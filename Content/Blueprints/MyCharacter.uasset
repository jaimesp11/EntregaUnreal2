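; Player character that handles Enhanced Input movement, look, jump and a pause menu, and holds health, score and stamina.
; BeginPlay creates the main UI, seeds its timer from MyGameMode and has the game mode place proofs.
; Left Shift sprints through RetriggerableDelay loops that set walk speed while draining or regenerating stamina.
; TakeDamage and IncreseScore adjust health and score; save-game creation logic is present but never runs.
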(event `self.ReceiveBeginPlay`
  (bind _asplayer_controller (cast `PlayerController` (`self.GetController`)))
  (message `EnhancedInputSubsystemInterface.AddMappingContext` (pcsubsystem `EnhancedInputLocalPlayerSubsystem` _asplayer_controller) "/Game/Input/MyMappingContext.MyMappingContext" 0 (struct))
  (bind _returnvalue (`|CreateWidget` "/Game/Blueprints/MyUI.MyUI_C" (`GameplayStatics.GetPlayerController` 0)))
  (bind _output_get (set `self.MainUI` _returnvalue))
  (bind _asmy_game_mode (cast `/Game/Blueprints/MyGameMode` (`GameplayStatics.GetGameMode`)))
  (`/Game/Blueprints/MyUI.UpdateTimeUI` _output_get (`/Game/Blueprints/MyGameMode.TimerMinutes` _asmy_game_mode) (`/Game/Blueprints/MyGameMode.TimerSeconds` _asmy_game_mode))
  (`UserWidget.AddToViewport` _returnvalue 0)
  (bind _asmy_game_mode_2 (cast `/Game/Blueprints/MyGameMode` (`GameplayStatics.GetGameMode`)))
  (`/Game/Blueprints/MyGameMode.PlaceProofs` _asmy_game_mode_2))

(event `EnhancedInput|/Game/Input/Action_Jump`
  (params (ActionValue :type Boolean) (ElapsedSeconds :type "Float (double-precision)") (TriggeredSeconds :type "Float (double-precision)") (InputAction :type "InputAction Object Reference" :default "/Game/Input/Action_Jump.Action_Jump"))
  (:`Started`
    (`self.Jump`))
  (:`Completed`
    (`self.StopJumping`)))

(event `EnhancedInput|/Game/Input/Action_Movement`
  (params (ActionValue :type "Vector2D Structure") (ElapsedSeconds :type "Float (double-precision)") (TriggeredSeconds :type "Float (double-precision)") (InputAction :type "InputAction Object Reference" :default "/Game/Input/Action_Movement.Action_Movement"))
  (bind (_x _y) (`KismetMathLibrary.BreakVector2D` ActionValue))
  (:`Triggered`
    (`self.AddMovementInput` (+ (* _x (`self.GetActorForwardVector`)) (* _y (`self.GetActorRightVector`))) (`KismetMathLibrary.VSize2D` ActionValue))))

(event `EnhancedInput|/Game/Input/Action_CameraMovemnet`
  (params (ActionValue :type "Vector2D Structure") (ElapsedSeconds :type "Float (double-precision)") (TriggeredSeconds :type "Float (double-precision)") (InputAction :type "InputAction Object Reference" :default "/Game/Input/Action_CameraMovemnet.Action_CameraMovemnet"))
  (:`Triggered`
    (`self.AddControllerYawInput` ActionValue_X)
    (`self.AddControllerPitchInput` (* ActionValue_Y -1.0))))

(event `EnhancedInput|/Game/Input/Action_Pause`
  (params (ActionValue :type Boolean) (ElapsedSeconds :type "Float (double-precision)") (TriggeredSeconds :type "Float (double-precision)") (InputAction :type "InputAction Object Reference" :default "/Game/Input/Action_Pause.Action_Pause"))
  (bind _returnvalue (`GameplayStatics.GetPlayerController` 0))
  (:`Started`
    (if (not (`self.IsPauseMenuOpened?`))
      (set `self.IsPauseMenuOpened?` true)
      (bind _returnvalue_2 (`|CreateWidget` "/Game/Blueprints/PauseMenu.PauseMenu_C" _returnvalue))
      (bind _output_get (set `self.PauseMenuWidget` _returnvalue_2))
      (`UserWidget.AddToViewport` _output_get 0)
      (`WidgetBlueprintLibrary.SetInputMode_GameAndUIEx` _returnvalue (`self.PauseMenuWidget`))
      (set `PlayerController.bShowMouseCursor` true _returnvalue)
      (`GameplayStatics.SetGamePaused` true)
      (else
        (set `self.IsPauseMenuOpened?` false)
        (`Widget.RemoveFromParent` (`self.PauseMenuWidget`))
        (`GameplayStatics.SetGamePaused` false)
        (`WidgetBlueprintLibrary.SetInputMode_GameOnly` _returnvalue)
        (set `PlayerController.bShowMouseCursor` false _returnvalue)))))

(event `Key|LeftShift`
  (params (Key :type "Key Structure"))
  (bind _charactermovement (`self.CharacterMovement`))
  (:`Pressed`
    (set `self.IsRunning?` true)
    (set `CharacterMovementComponent.MaxWalkSpeed` 1000.0 _charactermovement :!label _label)
    (`KismetSystemLibrary.RetriggerableDelay` 0.2)
    (`self.UseStamina`)
    (if (`self.IsRunning?`)
      (goto _label)))
  (:`Released`
    (set `self.IsRunning?` false)
    (set `CharacterMovementComponent.MaxWalkSpeed` 500.0 _charactermovement :!label _label_2)
    (`KismetSystemLibrary.RetriggerableDelay` 0.2)
    (`self.IncreaseStamina`)
    (if (`self.CanIncreaseStamina?`)
      (goto _label_2))))

(event `UseStamina`
  (set `self.Stamina` (- (`self.Stamina`) 2.0))
  (if (<= (`self.Stamina`) 0.0)
    (set `self.IsRunning?` false)
    (set `CharacterMovementComponent.MaxWalkSpeed` 600.0 (`self.CharacterMovement`))))

(event `IncreaseStamina`
  (if (not (`self.IsRunning?`))
    (set `self.Stamina` (+ (`self.Stamina`) 2.0))
    (if (>= (`self.Stamina`) 100.0)
      (set `self.CanIncreaseStamina?` false)
      (else
        (set `self.CanIncreaseStamina?` true)))))

(fn `IncreseScore`
  (params (ScoreAmount :type Integer))
  (set `self.Score` (+ ScoreAmount (`self.Score`))))

(fn `TakeDamage`
  (params (Damage :type "Float (double-precision)"))
  (set `self.Health` (+ (* Damage -1.0) (`self.Health`))))

(fn `UserConstructionScript`)