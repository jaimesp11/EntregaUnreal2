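; Bullet is a projectile actor that flies forward and damages the player character on contact.
; Tick moves it along its forward vector at Speed, scaled by delta time, using a swept SetActorLocation.
; On overlap it calls TakeDamage on a MyCharacter with a fixed amount, then destroys itself whatever it hit.
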(event `self.ReceiveActorBeginOverlap`
  (params (OtherActor :type "Actor Object Reference"))
  (bind _asmy_character (cast `/Game/Blueprints/MyCharacter` OtherActor)
    (:`then`
      (`/Game/Blueprints/MyCharacter.TakeDamage` _asmy_character 20.0))
    (:`CastFailed`
      _))
  (`self.K2_DestroyActor`))

(event `self.ReceiveTick`
  (params (DeltaSeconds :type "Float (single-precision)"))
  (`self.K2_SetActorLocation` (+ (`self.K2_GetActorLocation`) (* DeltaSeconds (* (`self.Speed`) (`self.GetActorForwardVector`)))) true))

(fn `UserConstructionScript`)