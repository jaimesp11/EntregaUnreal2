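; Game mode for a timed proof-hunting level, handling the countdown, save slots and item placement.
; BeginPlay starts a looping one-second timer that updates the character's UI and shows a losing EndScreen at zero.
; It also restores the character mesh transform or creates a save, though existence checks use "save1" while reads and writes use an empty slot name.
; PlaceProofs spawns proofs at random unused ProofSpawn actors, registers them in the UI, then destroys all spawners.
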(event `RestartLevel`
  ;[1 1 1] Delete Save + Restart
  (`GameplayStatics.DeleteGameInSlot` "save1")
  (`KismetSystemLibrary.ExecuteConsoleCommand` "RestartLevel" null))

(event `Load Game`
  ;[1 1 1] Load Game
  (`KismetSystemLibrary.ExecuteConsoleCommand` "RestartLevel" null))

(event `Savegame`
  ;[1 1 1] Save Game
  (bind _returnvalue (`GameplayStatics.LoadGameFromSlot` ""))
  (bind _asmy_save_game (cast `/Game/Blueprints/MySaveGame` _returnvalue))
  (set `/Game/Blueprints/MySaveGame.CharTransform` (`self.GetTransform` (cast `/Game/Blueprints/MyCharacter` (`GameplayStatics.GetPlayerCharacter` 0) :!pure true)) _asmy_save_game)
  (`GameplayStatics.SaveGameToSlot` _asmy_save_game))

(event `self.ReceiveBeginPlay`
  ;[1 1 1] Inicio partida
  (`self.StartCountDownTimer`)
  (`GameplayStatics.DoesSaveGameExist` "save1")
  (if true
    ;[1 1 1] Loadgame functionality
    (bind _returnvalue (`GameplayStatics.LoadGameFromSlot` ""))
    (bind _asmy_save_game (cast `/Game/Blueprints/MySaveGame` _returnvalue))
    (bind _asmy_character (cast `/Game/Blueprints/MyCharacter` (`GameplayStatics.GetPlayerCharacter` 0)))
    (`SceneComponent.K2_SetWorldTransform` (`Character.Mesh` _asmy_character) (`/Game/Blueprints/MySaveGame.CharTransform` _asmy_save_game) false false)
    (else
      ;[1 1 1] Create Savegame
      (bind _returnvalue_2 (`GameplayStatics.CreateSaveGameObject` "/Game/Blueprints/MySaveGame.MySaveGame_C"))
      (`GameplayStatics.SaveGameToSlot` _returnvalue_2))))

(event `StartCountDownTimer`
  ;[1 1 1] Temporizador
  (`KismetSystemLibrary.K2_SetTimerDelegate` (delegate `CountdownTimer`) 1.0 true))

(event `CountdownTimer`
  ;[1 1 1] Temporizador
  (bind _asmy_character (cast `/Game/Blueprints/MyCharacter` (`GameplayStatics.GetPlayerCharacter` 0)))
  (`/Game/Blueprints/MyUI.UpdateTimeUI` (`/Game/Blueprints/MyCharacter.MainUI` _asmy_character) (`self.TimerMinutes`) (`self.TimerSeconds`))
  (set `self.TimerSeconds` (- (`self.TimerSeconds`) 1))
  (if (< (`self.TimerSeconds`) 0)
    (if (== (`self.TimerMinutes`) 0)
      ;[1 1 1] Finalizar partida (jugador pierde) si se acaba temporizador
      (bind _returnvalue (`|CreateWidget` "/Game/Blueprints/EndScreen.EndScreen_C" (`GameplayStatics.GetPlayerController` 0)))
      (bind _output_get (set `self.EndScreen` _returnvalue))
      (`/Game/Blueprints/EndScreen.UpdateResultUI` (`self.EndScreen`) false)
      (`/Game/Blueprints/EndScreen.UpdateResultUI` _output_get false)
      (`UserWidget.AddToViewport` _returnvalue 0)
      (bind _asmy_character_2 (cast `/Game/Blueprints/MyCharacter` (`GameplayStatics.GetPlayerCharacter` 0)))
      (bind _mainui (`/Game/Blueprints/MyCharacter.MainUI` _asmy_character_2))
      (`/Game/Blueprints/MyUI.SaveGameStats` _mainui)
      (`KismetSystemLibrary.Delay` 0.2)
      (`Widget.RemoveFromParent` _mainui)
      (else
        (set `self.TimerMinutes` (- (`self.TimerMinutes`) 1))
        (set `self.TimerSeconds` 59)))))

(event `PlaceProofs`
  ;[1 1 1] Spawn Items
  (`KismetSystemLibrary.Delay` 0.5)
  (bind _outactors (`GameplayStatics.GetAllActorsOfClass` "/Game/Blueprints/ProofSpawn.ProofSpawn_C"))
  (set `self.ProofSpawners` _outactors)
  (`KismetSystemLibrary.PrintText` (`|FormatText` "Spawners forund: {SP}" (`KismetTextLibrary.Conv_IntToText` (`KismetArrayLibrary.Array_Length` (`self.ProofSpawners`)))) true true (struct :`R` 0.44615 :`G` 1.0 :`A` 1.0))
  (for (_array_element _array_index) (`self.ProofsNames`)
    (`self.ChooseRandomPlacement`)
    (while (`/Game/Blueprints/ProofSpawn.taken` (`self.CurrentProofSpawn`))
      (`self.ChooseRandomPlacement`))
    (bind _returnvalue (`|SpawnActorFromClass` (`self.ProofBlueprint`) (`self.GetTransform` (`self.CurrentProofSpawn`)) "AdjustIfPossibleButAlwaysSpawn" "MultiplyWithRoot" null null))
    (bind _asmy_character (cast `/Game/Blueprints/MyCharacter` (`GameplayStatics.GetPlayerCharacter` 0)))
    (bind _asproof__template (cast `/Game/Blueprints/Proof-Template` _returnvalue))
    (set `/Game/Blueprints/Proof-Template.ObjectName` _array_element _asproof__template)
    (set `/Game/Blueprints/Proof-Template.ObjectIndex` _array_index _asproof__template)
    (bind _output_get (set `/Game/Blueprints/Proof-Template.ProofImage` (`|GetArrayItem` (`self.ProofTextures`)) _asproof__template))
    (`/Game/Blueprints/MyUI.AddProofToFind` (`/Game/Blueprints/MyCharacter.MainUI` _asmy_character) _output_get)
    (set `/Game/Blueprints/ProofSpawn.taken` true (`self.CurrentProofSpawn`)))
  (`self.DestroySpawners`))

(event `ChooseRandomPlacement`
  (bind _proofspawners (`self.ProofSpawners`))
  ;[1 1 1] Spawn Items
  (set `self.CurrentProofSpawn` (`|GetArrayItem` _proofspawners (`KismetMathLibrary.RandomInteger` (`KismetArrayLibrary.Array_Length` _proofspawners)))))

(event `DestroySpawners`
  (for _array_element (`self.ProofSpawners`)
    (`self.K2_DestroyActor` _array_element)))

(fn `UserConstructionScript`)